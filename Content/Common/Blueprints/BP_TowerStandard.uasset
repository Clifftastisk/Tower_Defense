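; Standard tower Blueprint for a tower defense game that automatically shoots at the closest enemy in range.
; On BeginPlay it reads the "Tower1" data table row to set its detection sphere radius and start a looping fire-rate timer.
; Each shot picks the nearest overlapping enemy character, spawns a standard projectile with that enemy as target and plays a sound.
; Projectile behavior is left to the projectile Blueprint.
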(event `self.ReceiveBeginPlay`
  ;[1 0.02 0.02] Gathers information from Tower Data Table and establishes the range and firerate, based off of the data, for this specific tower
  (bind _returnvalue (`|GetDataTableRow` "/Game/Core/Data/TowerDataTable.TowerDataTable" "Tower1")
    (:`then`
      (`SphereComponent.SetSphereRadius` (`self.Sphere`) (`.Range_10_CE73546F44EA49D2C9C986B0A4451036` (break `/Game/Core/Data/TowerStruct` _returnvalue)) true)
      (`KismetSystemLibrary.K2_SetTimerDelegate` (delegate `FireStrd`) (`.Firerate_9_4E09FFD54CEB9780E5DE6C9E9C06523E` (break `/Game/Core/Data/TowerStruct` _returnvalue)) true))))

(event `FireStrd`
  ;[1 0.02 0.02] Fire projectile function for the tower. Gets the closest target within the radius and spawns a projectile. Projectile logic is then done in the projectile blueprint.
  (bind _targets (`self.GetClosestTarget` (`self.GetOverlappingActors` "/Game/Core/Blueprints/Bp_EnemyCharacter.Bp_EnemyCharacter_C")))
  (bind _asbp_enemy_character (cast `/Game/Core/Blueprints/Bp_EnemyCharacter` _targets))
  (`|SpawnActorFromClass` "/Game/Core/Blueprints/BP_ProcetileStandard.BP_ProcetileStandard_C" (`self.GetTransform`) "Undefined" "OverrideRootScale" null _asbp_enemy_character null)
  (`GameplayStatics.PlaySoundAtLocation` "/Game/Common/Sounds/ProjectileSound.ProjectileSound" (`self.K2_GetActorLocation`) (struct) 1.0 1.0 0.0 null null null))

(fn `GetClosestTarget`
  (params (EnemyArray :type "Array of Actor Object Reference"))
  (returns (Targets :type "Actor Object Reference"))
  (locals (TempDistance :type "Float (double-precision)") (TempTarget :type "Actor Object Reference"))
  ;[0.66 0.3934 0] Gets the closest target based off of the distance to other actors within the radius of the tower
  (for _array_element EnemyArray
    (`local.TempTarget`
      (:`then`
        (bind _returnvalue (`self.GetDistanceTo` _array_element))
        (if (< _returnvalue (`local.TempDistance`))
          (set `local.TempTarget` _array_element)
          (set `local.TempDistance` _returnvalue)))
      (:`else`
        (set `local.TempTarget` _array_element)
        (set `local.TempDistance` (`self.GetDistanceTo` _array_element)))))
  (return (`local.TempTarget`)))

(fn `UserConstructionScript`)