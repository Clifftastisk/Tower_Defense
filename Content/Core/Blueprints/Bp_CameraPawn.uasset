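; Camera pawn that gives the player free movement over the level and clicking on widgets.
; BeginPlay places it at a fixed elevated position with a set pitch.
; Tick polls player 0's keys directly: WASD moves it along world X/Y in fixed per-frame steps, unscaled by delta time, and mouse wheel input adjusts height.
; Left mouse press and release are forwarded to a WidgetInteraction component as pointer clicks.
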(event `self.ReceiveBeginPlay`
  (`self.K2_SetActorLocationAndRotation` (-762.0 -62.0 2100.0) (`KismetMathLibrary.MakeRotator` 0.0 20.0)))

(event `self.ReceiveTick`
  (params (DeltaSeconds :type "Float (single-precision)"))
  (bind (_returnvalue_x _returnvalue_y _returnvalue_z) (`KismetMathLibrary.BreakVector` (`self.K2_GetActorLocation`)))
  (bind (_returnvalue_x_2 _returnvalue_y_2 _returnvalue_z_2) (`KismetMathLibrary.BreakVector` (`self.K2_GetActorLocation`)))
  (bind (_returnvalue_x_3 _returnvalue_y_3 _returnvalue_z_3) (`KismetMathLibrary.BreakVector` (`self.K2_GetActorLocation`)))
  (bind (_returnvalue_x_4 _returnvalue_y_4 _returnvalue_z_4) (`KismetMathLibrary.BreakVector` (`self.K2_GetActorLocation`)))
  (bind (_returnvalue_x_5 _returnvalue_y_5 _returnvalue_z_5) (`KismetMathLibrary.BreakVector` (`self.K2_GetActorLocation`)))
  (`|ExecutionSequence`
    (:`then_0`
      (if (`PlayerController.IsInputKeyDown` (`GameplayStatics.GetPlayerController` 0) "D")
        (`self.K2_SetActorLocation` (`KismetMathLibrary.MakeVector` _returnvalue_x (+ _returnvalue_y 20.0) _returnvalue_z))))
    (:`then_1`
      (if (`PlayerController.IsInputKeyDown` (`GameplayStatics.GetPlayerController` 0) "A")
        (`self.K2_SetActorLocation` (`KismetMathLibrary.MakeVector` _returnvalue_x_2 (- _returnvalue_y_2 20.0) _returnvalue_z_2))))
    (:`then_2`
      (if (`PlayerController.IsInputKeyDown` (`GameplayStatics.GetPlayerController` 0) "W")
        (`self.K2_SetActorLocation` (`KismetMathLibrary.MakeVector` (+ _returnvalue_x_5 20.0) _returnvalue_y_5 _returnvalue_z_5))))
    (:`then_3`
      (if (`PlayerController.IsInputKeyDown` (`GameplayStatics.GetPlayerController` 0) "S")
        (`self.K2_SetActorLocation` (`KismetMathLibrary.MakeVector` (- _returnvalue_x_3 20.0) _returnvalue_y_3 _returnvalue_z_3))))
    (:`then_4`
      (if (`PlayerController.IsInputKeyDown` (`GameplayStatics.GetPlayerController` 0) "MouseWheelAxis")
        (`self.K2_SetActorLocation` (`KismetMathLibrary.MakeVector` _returnvalue_x_4 _returnvalue_y_4 (+ _returnvalue_z_4 (`self.GetInputAxisKeyValue`))))))))

(event `Key|LeftMouseButton`
  (params (Key :type "Key Structure"))
  (:`Pressed`
    (`WidgetInteractionComponent.PressPointerKey` (`self.WidgetInteraction`) "LeftMouseButton"))
  (:`Released`
    (`WidgetInteractionComponent.ReleasePointerKey` (`self.WidgetInteraction`) "LeftMouseButton")))

(fn `UserConstructionScript`)