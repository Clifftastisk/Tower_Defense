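; BP_ProcetileHoming is a homing tower projectile that damages the enemy it hits.
; Tick moves it toward EnemyCheck with constant-speed interpolation and destroys it after a five-second delay.
; On overlap it looks up the hard-coded Tower2 row in TowerDataTable, subtracts Damage from the enemy's Health, destroys itself and calls CheckIsDead.
; Tick's speed comes from that same row lookup, which only executes on overlap.
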(event `self.ReceiveActorBeginOverlap`
  (params (OtherActor :type "Actor Object Reference"))
  (bind _returnvalue (`|GetDataTableRow` "/Game/Core/Data/TowerDataTable.TowerDataTable" "Tower2")
    (:`then`
      (bind _asbp_enemy_character (cast `/Game/Core/Blueprints/Bp_EnemyCharacter` OtherActor))
      (set `/Game/Core/Blueprints/Bp_EnemyCharacter.Health` (- (`/Game/Core/Blueprints/Bp_EnemyCharacter.Health` _asbp_enemy_character) (break `/Game/Core/Data/TowerStruct` _returnvalue)) _asbp_enemy_character)
      (`self.K2_DestroyActor`)
      (`/Game/Core/Blueprints/Bp_EnemyCharacter.CheckIsDead` _asbp_enemy_character))))

(event `self.ReceiveTick`
  (params (DeltaSeconds :type "Float (single-precision)"))
  (`self.K2_SetActorLocation` (`KismetMathLibrary.VInterpTo_Constant` (`self.K2_GetActorLocation`) (`self.K2_GetActorLocation` (`self.EnemyCheck`)) DeltaSeconds (`.ProjectileSpeed_11_A9D969CD4FB872F9117F538A27158743` (break `/Game/Core/Data/TowerStruct` (stale `self.ReceiveActorBeginOverlap` _returnvalue)))))
  (`KismetSystemLibrary.Delay` 5.0)
  (`self.K2_DestroyActor`))

(fn `UserConstructionScript`)