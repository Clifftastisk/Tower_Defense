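; Fire tower projectile that homes in on a target enemy and deals damage on overlap, using the Tower2 data table row.
; Tick moves it toward EnemyCheck at constant speed, reading ProjectileSpeed from the row lookup that only runs on overlap, and destroys it after a short delay.
; Overlapping an enemy character subtracts Health, updates its HP bar widget, runs its death check and destroys the projectile.
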(event `self.ReceiveActorBeginOverlap`
  (params (OtherActor :type "Actor Object Reference"))
  (bind _returnvalue (`|GetDataTableRow` "/Game/Core/Data/TowerDataTable.TowerDataTable" "Tower2")
    (:`then`
      (bind _asbp_enemy_character (cast `/Game/Core/Blueprints/Bp_EnemyCharacter` OtherActor))
      (set `/Game/Core/Blueprints/Bp_EnemyCharacter.Health` (- (`/Game/Core/Blueprints/Bp_EnemyCharacter.Health` _asbp_enemy_character) (break `/Game/Core/Data/TowerStruct` _returnvalue)) _asbp_enemy_character)
      (bind _output_get (set `self.WidHpRef` (`WidgetComponent.GetUserWidgetObject` (`/Game/Core/Blueprints/Bp_EnemyCharacter.Widget1` _asbp_enemy_character))))
      (bind _aswidget_enemy_hpbar (cast `/Game/Common/Widgets/Widget_EnemyHPBar` _output_get))
      (`/Game/Common/Widgets/Widget_EnemyHPBar.ModifyHealth` _aswidget_enemy_hpbar (break `/Game/Core/Data/TowerStruct` _returnvalue))
      (`/Game/Core/Blueprints/Bp_EnemyCharacter.CheckIsDead` _asbp_enemy_character)
      (`self.K2_DestroyActor`))))

(event `self.ReceiveTick`
  (params (DeltaSeconds :type "Float (single-precision)"))
  (`self.K2_SetActorLocation` (`KismetMathLibrary.VInterpTo_Constant` (`self.K2_GetActorLocation`) (`self.K2_GetActorLocation` (`self.EnemyCheck`)) DeltaSeconds (`.ProjectileSpeed_11_A9D969CD4FB872F9117F538A27158743` (break `/Game/Core/Data/TowerStruct` (stale `self.ReceiveActorBeginOverlap` _returnvalue)))))
  (`KismetSystemLibrary.Delay` 0.8)
  (`self.K2_DestroyActor`))

(fn `UserConstructionScript`)