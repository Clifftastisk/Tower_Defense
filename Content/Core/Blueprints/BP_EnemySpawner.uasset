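; Enemy wave spawner that runs three timed waves per level, then loads the next level or shows the win screen.
; BeginPlay reads per-wave standard, heavy and fast enemy counts from a DataTable and starts a looping countdown widget timer.
; Tick counts down, spawns enemies until live counts reach wave targets, and re-issues AIMoveTo toward FinishPoint to handle the dynamic navmesh.
; After the last wave, finding no enemies left triggers FinalWave.
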(event `self.ReceiveTick`
  (params (DeltaSeconds :type "Float (single-precision)"))
  (bind _finish_point (`self.Finish point`))
  (bind _standardamount_w2 (`self.StandardAmount W2`))
  (bind _finish_point_2 (`self.Finish point`))
  (bind _finish_point_3 (`self.Finish point`))
  (bind _standardamount_w3 (`self.StandardAmount W3`))
  ;[1 0.02 0.02] Every tick, send out prompts to move AI towards goal. Tick is needed because of the Gate System design; the navmesh is dynamic and allows the AI to change course, therefore there needs to be a a constant update. Also handles timer.
  (bind _output_get (set `self.WaveTime` (- (`self.WaveTime`) (`GameplayStatics.GetWorldDeltaSeconds`))))
  (`|ExecutionSequence`
    (:`then_0`
      ;[1 0.02 0.02] Wave 1 Spawn & Movement - Spawn logic for different waves
      (if (and (< (`self.WaveTime`) 1.0) (`self.Wave1Active`))
        (`|ExecutionSequence`
          (:`then_0`
            (bind _outactors (`GameplayStatics.GetAllActorsOfClass` "/Game/Common/Blueprints/BPI_EnemyStandard.BPI_EnemyStandard_C"))
            (if (< (`KismetArrayLibrary.Array_Length` _outactors) (`self.StandardAmount W1`))
              (`KismetSystemLibrary.Delay` 0.8)
              (bind _returnvalue (`AIBlueprintHelperLibrary.SpawnAIFromClass` "/Game/Common/Blueprints/BPI_EnemyStandard.BPI_EnemyStandard_C" null (`self.K2_GetActorLocation`) (struct) false null))
              (bind _outactors_2 (`GameplayStatics.GetAllActorsOfClass` "/Game/Common/Blueprints/BPI_EnemyStandard.BPI_EnemyStandard_C"))
              (`|ExecutionSequence`
                (:`then_0`
                  (if (== (`KismetArrayLibrary.Array_Length` _outactors_2) (`self.StandardAmount W1`))
                    (`self.ResetWaveCountdown`)
                    (set `self.Wave1Active` false)
                    (set `self.Wave2Active` true)
                    (set `self.WaveTime` 30.0))))))
          (:`then_1`
            (bind _outactors_3 (`GameplayStatics.GetAllActorsOfClass` "/Game/Common/Blueprints/BPI_EnemyHeavy.BPI_EnemyHeavy_C"))
            (if (< (`KismetArrayLibrary.Array_Length` _outactors_3) (`self.HeavyAmount W1`))
              (`KismetSystemLibrary.Delay` 0.8)
              (bind _returnvalue_2 (`AIBlueprintHelperLibrary.SpawnAIFromClass` "/Game/Common/Blueprints/BPI_EnemyHeavy.BPI_EnemyHeavy_C" null (`self.K2_GetActorLocation`) (struct) false null))))
          (:`then_2`
            (bind _outactors_4 (`GameplayStatics.GetAllActorsOfClass` "/Game/Common/Blueprints/BPI_EnemyFast.BPI_EnemyFast_C"))
            (if (< (`KismetArrayLibrary.Array_Length` _outactors_4) (`self.FastAmount W1`))
              (`KismetSystemLibrary.Delay` 0.8)
              (bind _returnvalue_3 (`AIBlueprintHelperLibrary.SpawnAIFromClass` "/Game/Common/Blueprints/BPI_EnemyFast.BPI_EnemyFast_C" null (`self.K2_GetActorLocation`) (struct) false null)))))))
    (:`then_1`
      (`KismetSystemLibrary.Delay` 0.2)
      (`|ExecutionSequence`
        (:`then_0`
          (`|AIMoveTo` _returnvalue (0.0 0.0 0.0) _finish_point_3 1.0
            (:`then`
              (`|AIMoveTo` _returnvalue_2 (0.0 0.0 0.0) _finish_point_3 1.0
                (:`then`
                  (`|AIMoveTo` _returnvalue_3 (0.0 0.0 0.0) _finish_point_3 1.0))))))
        (:`then_1`
          ;[1 0.02 0.02] Wave 2 Spawn & Movement - Spawn logic for different waves
          (`|AIMoveTo` (stale _returnvalue_4) (0.0 0.0 0.0) _finish_point_2 1.0
            (:`then`
              (`|AIMoveTo` (stale _returnvalue_6) (0.0 0.0 0.0) _finish_point_2 1.0
                (:`then`
                  (`|AIMoveTo` (stale _returnvalue_7) (0.0 0.0 0.0) _finish_point_2 1.0))))))
        (:`then_2`
          ;[1 0.02 0.02] Wave 3 Spawn & Movement - Spawn logic for different waves
          (`|AIMoveTo` (stale _returnvalue_8) (0.0 0.0 0.0) _finish_point 1.0
            (:`then`
              (`|AIMoveTo` (stale _returnvalue_10) (0.0 0.0 0.0) _finish_point 1.0
                (:`then`
                  (`|AIMoveTo` (stale _returnvalue_11) (0.0 0.0 0.0) _finish_point 1.0
                    (:`then`
                      ;;[1 1 1] LastWaveSpecial check
                      (if (`self.LastWave?`)
                        (`KismetSystemLibrary.Delay` 5.0)
                        (bind _outactors_5 (`GameplayStatics.GetAllActorsOfClass` "/Game/Common/Blueprints/BPI_EnemyStandard.BPI_EnemyStandard_C"))
                        (bind _outactors_6 (`GameplayStatics.GetAllActorsOfClass` "/Game/Common/Blueprints/BPI_EnemyHeavy.BPI_EnemyHeavy_C"))
                        (bind _outactors_7 (`GameplayStatics.GetAllActorsOfClass` "/Game/Common/Blueprints/BPI_EnemyFast.BPI_EnemyFast_C"))
                        (if (and (== (`KismetArrayLibrary.Array_Length` _outactors_5) 0) (== (`KismetArrayLibrary.Array_Length` _outactors_6) 0))
                          (if (== (`KismetArrayLibrary.Array_Length` _outactors_7) 0)
                            (`self.FinalWave`)))))))))))))
    (:`then_2`
      (if (and (< (`self.WaveTime`) 1.0) (`self.Wave2Active`))
        (`|ExecutionSequence`
          (:`then_0`
            (bind _outactors_8 (`GameplayStatics.GetAllActorsOfClass` "/Game/Common/Blueprints/BPI_EnemyStandard.BPI_EnemyStandard_C"))
            (if (< (`KismetArrayLibrary.Array_Length` _outactors_8) (+ (`self.StandardAmount W1`) (`self.StandardAmount W2`)))
              (`KismetSystemLibrary.Delay` 0.8)
              (bind _returnvalue_4 (`AIBlueprintHelperLibrary.SpawnAIFromClass` "/Game/Common/Blueprints/BPI_EnemyStandard.BPI_EnemyStandard_C" null (`self.K2_GetActorLocation`) (struct) false null))
              (bind _outactors_9 (`GameplayStatics.GetAllActorsOfClass` "/Game/Common/Blueprints/BPI_EnemyStandard.BPI_EnemyStandard_C"))
              (bind _returnvalue_5 (`KismetArrayLibrary.Array_Length` _outactors_9))
              (if (or (>= _returnvalue_5 (+ (`self.StandardAmount W1`) _standardamount_w2)) (== _returnvalue_5 _standardamount_w2))
                (`self.ResetWaveCountdown`)
                (set `self.Wave2Active` false)
                (set `self.Wave3Active` true)
                (set `self.WaveTime` 30.0))))
          (:`then_1`
            (bind _outactors_10 (`GameplayStatics.GetAllActorsOfClass` "/Game/Common/Blueprints/BPI_EnemyHeavy.BPI_EnemyHeavy_C"))
            (if (< (`KismetArrayLibrary.Array_Length` _outactors_10) (+ (`self.HeavyAmount W1`) (`self.HeavyAmount W2`)))
              (`KismetSystemLibrary.Delay` 0.8)
              (bind _returnvalue_6 (`AIBlueprintHelperLibrary.SpawnAIFromClass` "/Game/Common/Blueprints/BPI_EnemyHeavy.BPI_EnemyHeavy_C" null (`self.K2_GetActorLocation`) (struct) false null))))
          (:`then_2`
            (bind _outactors_11 (`GameplayStatics.GetAllActorsOfClass` "/Game/Common/Blueprints/BPI_EnemyFast.BPI_EnemyFast_C"))
            (if (< (`KismetArrayLibrary.Array_Length` _outactors_11) (+ (`self.FastAmount W1`) (`self.FastAmount W2`)))
              (`KismetSystemLibrary.Delay` 0.8)
              (bind _returnvalue_7 (`AIBlueprintHelperLibrary.SpawnAIFromClass` "/Game/Common/Blueprints/BPI_EnemyFast.BPI_EnemyFast_C" null (`self.K2_GetActorLocation`) (struct) false null)))))))
    (:`then_3`
      (if (and (< (`self.WaveTime`) 1.0) (`self.Wave3Active`))
        (`|ExecutionSequence`
          (:`then_0`
            (bind _outactors_12 (`GameplayStatics.GetAllActorsOfClass` "/Game/Common/Blueprints/BPI_EnemyStandard.BPI_EnemyStandard_C"))
            (if (< (`KismetArrayLibrary.Array_Length` _outactors_12) (+ (`self.StandardAmount W2`) (`self.StandardAmount W3`)))
              (`KismetSystemLibrary.Delay` 0.8)
              (bind _returnvalue_8 (`AIBlueprintHelperLibrary.SpawnAIFromClass` "/Game/Common/Blueprints/BPI_EnemyStandard.BPI_EnemyStandard_C" null (`self.K2_GetActorLocation`) (struct) false null))
              (bind _outactors_13 (`GameplayStatics.GetAllActorsOfClass` "/Game/Common/Blueprints/BPI_EnemyStandard.BPI_EnemyStandard_C"))
              (bind _returnvalue_9 (`KismetArrayLibrary.Array_Length` _outactors_13))
              (if (or (>= _returnvalue_9 (+ (`self.StandardAmount W2`) _standardamount_w3)) (== _returnvalue_9 _standardamount_w3))
                (set `self.Wave3Active` false)
                (set `self.LastWave?` true))))
          (:`then_1`
            (bind _outactors_14 (`GameplayStatics.GetAllActorsOfClass` "/Game/Common/Blueprints/BPI_EnemyHeavy.BPI_EnemyHeavy_C"))
            (if (< (`KismetArrayLibrary.Array_Length` _outactors_14) (+ (`self.HeavyAmount W2`) (`self.HeavyAmount W3`)))
              (`KismetSystemLibrary.Delay` 0.8)
              (bind _returnvalue_10 (`AIBlueprintHelperLibrary.SpawnAIFromClass` "/Game/Common/Blueprints/BPI_EnemyHeavy.BPI_EnemyHeavy_C" null (`self.K2_GetActorLocation`) (struct) false null))))
          (:`then_2`
            (bind _outactors_15 (`GameplayStatics.GetAllActorsOfClass` "/Game/Common/Blueprints/BPI_EnemyFast.BPI_EnemyFast_C"))
            (if (< (`KismetArrayLibrary.Array_Length` _outactors_15) (+ (`self.FastAmount W2`) (`self.FastAmount W3`)))
              (`KismetSystemLibrary.Delay` 0.8)
              (bind _returnvalue_11 (`AIBlueprintHelperLibrary.SpawnAIFromClass` "/Game/Common/Blueprints/BPI_EnemyFast.BPI_EnemyFast_C" null (`self.K2_GetActorLocation`) (struct) false null)))))))
    (:`then_4`
      (if (== _output_get 30.0)
        (`self.WaveCountdown`)))))

(event `ResetWaveCountdown`
  ;[0.66 0.3934 0] When triggered, the even changes the widget colour to green and depending on the wave resets WaveCountdown.
  (`TextBlock.SetColorAndOpacity` (`/Game/Common/Widgets/Widget_Waves.WaveCountdown` (`self.WidgetWaveReference`)) (make `SlateColor` (struct :`R` 0.057249 :`G` 1.0 :`A` 1.0)))
  (`|ExecutionSequence`
    (:`then_0`
      (if (`self.Wave1Active`)
        (`KismetSystemLibrary.K2_UnPauseTimer` null "WaveCountdown")))
    (:`then_1`
      (if (`self.Wave2Active`)
        (`KismetSystemLibrary.K2_UnPauseTimer` null "WaveCountdown")))
    (:`then_2`
      (if (`self.Wave3Active`)
        (`KismetSystemLibrary.K2_UnPauseTimer` null "WaveCountdown")))))

(event `FinalWave`
  (bind _widgetwavereference (`self.WidgetWaveReference`))
  ;[0.2705 0.88 1] FinalWave function. Handles widget specifics
  (`TextBlock.SetOpacity` (`/Game/Common/Widgets/Widget_Waves.Completed` _widgetwavereference) 1.0)
  (`TextBlock.SetOpacity` (`/Game/Common/Widgets/Widget_Waves.WaveText` _widgetwavereference) 0.0)
  (`TextBlock.SetOpacity` (`/Game/Common/Widgets/Widget_Waves.WaveNr` _widgetwavereference) 0.0)
  (`TextBlock.SetOpacity` (`/Game/Common/Widgets/Widget_Waves.WaveCountdown` _widgetwavereference) 0.0)
  (`|ExecutionSequence`
    (:`then_0`
      (if (`self.Level 1`)
        (`GameplayStatics.OpenLevel` "L_2")
        (bind _foundwidgets (`WidgetBlueprintLibrary.GetAllWidgetsOfClass` "/Game/Common/Widgets/Widget_money.Widget_money_C"))
        (set `/Game/Common/Widgets/Widget_money.MoneyInTheMnyWidg` 0 (`|GetArrayItem` _foundwidgets))
        (`self.K2_DestroyActor`)))
    (:`then_1`
      (if (`self.Level 2`)
        (`GameplayStatics.OpenLevel` "L_3")
        (bind _foundwidgets_2 (`WidgetBlueprintLibrary.GetAllWidgetsOfClass` "/Game/Common/Widgets/Widget_money.Widget_money_C"))
        (set `/Game/Common/Widgets/Widget_money.MoneyInTheMnyWidg` 0 (`|GetArrayItem` _foundwidgets_2))
        (`self.K2_DestroyActor`)))
    (:`then_2`
      (if (`self.Level 3`)
        (bind _returnvalue (`|CreateWidget` "/Game/Common/Widgets/Widget_Winscreen.Widget_Winscreen_C"))
        (`UserWidget.AddToViewport` _returnvalue 0)
        (`KismetSystemLibrary.Delay` 5.0)
        (`GameplayStatics.OpenLevel` "L_0_Menu")))))

(event `self.ReceiveBeginPlay`
  ;[1 0.02 0.02] Establish local variables with the values gathered from Data tables. The Data tables are modular and can be edited by name in the editor.
  (`|ExecutionSequence`
    (:`then_0`
      (bind _returnvalue (`|CreateWidget` "/Game/Common/Widgets/Widget_Waves.Widget_Waves_C"))
      (bind _output_get (set `self.WidgetWaveReference` _returnvalue))
      (`UserWidget.AddToViewport` _output_get 0)
      ;[0.2705 0.88 1] After all variables have been established. Run a wave countdown function that updates the Core Widgets time (30 seconds - 1). This event is checked every 0.3 seconds for optimization.
      (`KismetSystemLibrary.K2_SetTimerDelegate` (delegate `WaveCountdown`) 0.3 true))
    (:`then_1`
      (bind _returnvalue_2 (`|GetDataTableRow` "/Game/Core/Data/SpawnerDataTable.SpawnerDataTable" (`self.Wave1`))
        (:`then`
          (`|ExecutionSequence`
            (:`then_0`
              (set `self.StandardAmount W1` (break `/Game/Core/Data/SpawnStructure` _returnvalue_2)))
            (:`then_1`
              (set `self.HeavyAmount W1` (`.HeavyAmount_11_A8EB2206471ACB333DCEA7840CAFF15A` (break `/Game/Core/Data/SpawnStructure` _returnvalue_2))))
            (:`then_2`
              (set `self.FastAmount W1` (`.FastAmount_12_A94A0F9649B44B39AD2E269AE7819D67` (break `/Game/Core/Data/SpawnStructure` _returnvalue_2)))
              (bind _returnvalue_3 (`|GetDataTableRow` "/Game/Core/Data/SpawnerDataTable.SpawnerDataTable" (`self.Wave2`))
                (:`then`
                  (`|ExecutionSequence`
                    (:`then_0`
                      (set `self.StandardAmount W2` (break `/Game/Core/Data/SpawnStructure` _returnvalue_3)))
                    (:`then_1`
                      (set `self.HeavyAmount W2` (`.HeavyAmount_11_A8EB2206471ACB333DCEA7840CAFF15A` (break `/Game/Core/Data/SpawnStructure` _returnvalue_3))))
                    (:`then_2`
                      (set `self.FastAmount W2` (`.FastAmount_12_A94A0F9649B44B39AD2E269AE7819D67` (break `/Game/Core/Data/SpawnStructure` _returnvalue_3)))
                      (bind _returnvalue_4 (`|GetDataTableRow` "/Game/Core/Data/SpawnerDataTable.SpawnerDataTable" (`self.Wave3`))
                        (:`then`
                          (`|ExecutionSequence`
                            (:`then_0`
                              (set `self.StandardAmount W3` (break `/Game/Core/Data/SpawnStructure` _returnvalue_4)))
                            (:`then_1`
                              (set `self.HeavyAmount W3` (`.HeavyAmount_11_A8EB2206471ACB333DCEA7840CAFF15A` (break `/Game/Core/Data/SpawnStructure` _returnvalue_4))))
                            (:`then_2`
                              (set `self.FastAmount W3` (`.FastAmount_12_A94A0F9649B44B39AD2E269AE7819D67` (break `/Game/Core/Data/SpawnStructure` _returnvalue_4))))))))))))))))))

(event `WaveCountdown`
  ;[0.2705 0.88 1] After all variables have been established. Run a wave countdown function that updates the Core Widgets time (30 seconds - 1). This event is checked every 0.3 seconds for optimization.
  (`TextBlock.SetText` (`/Game/Common/Widgets/Widget_Waves.WaveCountdown` (stale `self.ReceiveBeginPlay` _output_get)) (`KismetTextLibrary.Conv_IntToText` (`KismetMathLibrary.FTrunc` (`self.WaveTime`))))
  (if (< (`self.WaveTime`) 1.0)
    ;[0.2705 0.88 1] If Wave time = 0 the colour changes to red
    (`KismetSystemLibrary.K2_PauseTimer` null "WaveCountdown")
    (`TextBlock.SetColorAndOpacity` (`/Game/Common/Widgets/Widget_Waves.WaveCountdown` (`self.WidgetWaveReference`)) (make `SlateColor` (struct :`R` 1.0 :`B` 0.016184 :`A` 1.0)))
    ;[0.2705 0.88 1] If Wave time = 0 så add Wave to trigger by 1 and update widget.
    (bind _output_get (set `self.WhichWaveToTrigger` (+ (`self.WhichWaveToTrigger`) 1)))
    (`TextBlock.SetText` (`/Game/Common/Widgets/Widget_Waves.WaveNr` (`self.WidgetWaveReference`)) (`KismetTextLibrary.Conv_IntToText` _output_get))))

(fn `UserConstructionScript`)