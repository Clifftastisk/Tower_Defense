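; Player controller that runs the passive money income and handles cancelling build mode.
; On BeginPlay it hides on-screen debug messages, adds the money widget to the viewport and starts a looping timer that periodically increments the money total.
; The money value is stored directly on the widget rather than in the controller.
; Right mouse button fires the CancelBuildMode call and clears the build-mode flag.
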(event `self.ReceiveBeginPlay`
  (`KismetSystemLibrary.ExecuteConsoleCommand` "DisableAllScreenMessages" null)
  (bind _returnvalue (`|CreateWidget` "/Game/Common/Widgets/Widget_money.Widget_money_C"))
  (bind _output_get (set `self.MoneyReferenceWid` _returnvalue))
  (`UserWidget.AddToViewport` _output_get 0)
  (`KismetSystemLibrary.K2_SetTimerDelegate` (delegate `addmoney`) 0.5 true))

(event `Key|RightMouseButton`
  (params (Key :type "Key Structure"))
  (:`Pressed`
    (`self.CancelBuildMode`)
    (set `self.BuildModeActive` false)))

(event `addmoney`
  (set `/Game/Common/Widgets/Widget_money.MoneyInTheMnyWidg` (+ (`/Game/Common/Widgets/Widget_money.MoneyInTheMnyWidg` (stale `self.ReceiveBeginPlay` _output_get)) 2) (stale `self.ReceiveBeginPlay` _output_get)))

(fn `UserConstructionScript`)