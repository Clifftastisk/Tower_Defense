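; Base enemy character with a health bar, a death check and a slow effect.
; Tick rotates the widget to face the player camera, and CheckIsDead plays a death sound and destroys the actor once Health drops below one.
; Slowed, triggered by the sludge projectile, reduces walk speed with a minimum clamp and blocks repeat slows for a short delay; the speed is never restored here.
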(event `self.ReceiveTick`
  (params (DeltaSeconds :type "Float (single-precision)"))
  ;[0.66 0.3934 0] HP Bar rotation towards camera
  (`SceneComponent.K2_SetWorldRotation` (`self.Widget1`) (`KismetMathLibrary.FindLookAtRotation` (`SceneComponent.K2_GetComponentLocation` (`self.Widget1`)) (`SceneComponent.K2_GetComponentLocation` (`PlayerCameraManager.TransformComponent` (`GameplayStatics.GetPlayerCameraManager` 0)))) false false))

(event `CheckIsDead`
  ;[1 0.02 0.02] Checks if a target is dead, if so play a sound and destroy actor
  (if (< (`self.Health`) 1.0)
    (`GameplayStatics.PlaySoundAtLocation` "/Game/Common/Sounds/DeathSound.DeathSound" (`self.K2_GetActorLocation`) (struct) 1.0 1.0 0.0 null null null)
    (`self.K2_DestroyActor`)))

(event `Slowed`
  (bind _charactermovement (`self.CharacterMovement`))
  (bind _slowamount (`self.SlowAmount`))
  (bind _maxwalkspeed (`CharacterMovementComponent.MaxWalkSpeed` _charactermovement))
  ;[0.66 0.3934 0] Slowing function that's called from the Slow/sludge projectile.
  (if (not (`self.IsSlowed`))
    (set `self.IsSlowed` true)
    (set `CharacterMovementComponent.MaxWalkSpeed` (`KismetMathLibrary.FClamp` (- _maxwalkspeed _slowamount) _slowamount _maxwalkspeed) _charactermovement)
    (`KismetSystemLibrary.Delay` 2.0)
    (set `self.IsSlowed` false)))

(fn `UserConstructionScript`)