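; BP_ProcetilSludge is a homing sludge projectile, apparently fired by a tower, that leaves a spill where it hits an enemy.
; Tick moves it toward EnemyCheck at constant speed, read from the Tower3 data table row that is only fetched in the overlap event.
; Overlapping a Bp_EnemyCharacter spawns BP_SludgeSpill at that enemy's location and destroys the projectile.
; A delay started from Tick destroys it after four seconds otherwise.
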(event `self.ReceiveActorBeginOverlap`
  (params (OtherActor :type "Actor Object Reference"))
  (bind _returnvalue (`|GetDataTableRow` "/Game/Core/Data/TowerDataTable.TowerDataTable" "Tower3")
    (:`then`
      (bind _asbp_enemy_character (cast `/Game/Core/Blueprints/Bp_EnemyCharacter` OtherActor))
      (`|SpawnActorFromClass` "/Game/Core/Blueprints/BP_SludgeSpill.BP_SludgeSpill_C" (`KismetMathLibrary.Conv_VectorToTransform` (`self.K2_GetActorLocation` _asbp_enemy_character)) "Undefined" "OverrideRootScale" null null)
      (`self.K2_DestroyActor`))))

(event `self.ReceiveTick`
  (params (DeltaSeconds :type "Float (single-precision)"))
  (`self.K2_SetActorLocation` (`KismetMathLibrary.VInterpTo_Constant` (`self.K2_GetActorLocation`) (`self.K2_GetActorLocation` (`self.EnemyCheck`)) DeltaSeconds (`.ProjectileSpeed_11_A9D969CD4FB872F9117F538A27158743` (break `/Game/Core/Data/TowerStruct` (stale `self.ReceiveActorBeginOverlap` _returnvalue)))))
  (`KismetSystemLibrary.Delay` 4.0)
  (`self.K2_DestroyActor`))

(fn `UserConstructionScript`)