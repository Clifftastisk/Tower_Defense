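; Wave spawner actor that counts down to an enemy wave and drives an on-screen wave widget.
; A looping timer decrements the countdown; at zero it pauses, updates the widget and triggers Wave1.
; Wave1 uses delayed timers to spawn two enemies at the actor's location, both standard class despite one event's Fast name.
; After a delay it shows Completed and destroys itself, as only one wave exists.
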(event `self.ReceiveBeginPlay`
  (bind _returnvalue (`|CreateWidget` "/Game/Common/Widgets/Widget_Waves.Widget_Waves_C"))
  (bind _output_get (set `self.WidgetWaveReference` _returnvalue))
  (`UserWidget.AddToViewport` _output_get 0)
  (`KismetSystemLibrary.K2_SetTimerDelegate` (delegate `CountUntilNextWave`) (`KismetMathLibrary.Conv_IntToDouble` (`self.WaveTimer`)) true))

(event `CountUntilNextWave`
  (bind _widgetwavereference (`self.WidgetWaveReference`))
  (bind _output_get (set `self.UntilNextWave` (- (`self.UntilNextWave`) 1)))
  (`TextBlock.SetText` (`/Game/Common/Widgets/Widget_Waves.WaveCountdown` (stale `self.ReceiveBeginPlay` _output_get)) (`KismetTextLibrary.Conv_IntToText` _output_get))
  (if (== (`self.UntilNextWave`) 0)
    (`KismetSystemLibrary.K2_PauseTimer` null "CountUntilNextWave")
    (`TextBlock.SetColorAndOpacity` (`/Game/Common/Widgets/Widget_Waves.WaveCountdown` (`self.WidgetWaveReference`)) (make `SlateColor` (struct :`R` 1.0 :`B` 0.016184 :`A` 1.0)))
    (bind _output_get_2 (set `self.WhichWaveToTrigger` (+ (`self.WhichWaveToTrigger`) 1)))
    (`TextBlock.SetText` (`/Game/Common/Widgets/Widget_Waves.WaveNr` (`self.WidgetWaveReference`)) (`KismetTextLibrary.Conv_IntToText` _output_get_2))
    (`|ExecutionSequence`
      (:`then_0`
        (if (== (`self.WhichWaveToTrigger`) 1)
          (`self.Wave1`)
          (`KismetSystemLibrary.Delay` 30.0)
          (set `self.UntilNextWave` 30)
          (`TextBlock.SetColorAndOpacity` (`/Game/Common/Widgets/Widget_Waves.WaveCountdown` (`self.WidgetWaveReference`)) (make `SlateColor` (struct :`R` 0.057249 :`G` 1.0 :`A` 1.0)))
          (if (== (`self.WhichWaveToTrigger`) 1)
            (`TextBlock.SetOpacity` (`/Game/Common/Widgets/Widget_Waves.Completed` _widgetwavereference) 1.0)
            (`TextBlock.SetOpacity` (`/Game/Common/Widgets/Widget_Waves.WaveText` _widgetwavereference) 0.0)
            (`TextBlock.SetOpacity` (`/Game/Common/Widgets/Widget_Waves.WaveNr` _widgetwavereference) 0.0)
            (`TextBlock.SetOpacity` (`/Game/Common/Widgets/Widget_Waves.WaveCountdown` _widgetwavereference) 0.0)
            (`self.K2_DestroyActor`)
            (else
              (`KismetSystemLibrary.K2_UnPauseTimer` null "CountUntilNextWave"))))))))

(event `Wave1`
  (`KismetSystemLibrary.K2_SetTimerDelegate` (delegate `SpawnStandardEnemy1`) 3.0)
  (`KismetSystemLibrary.K2_SetTimerDelegate` (delegate `SpawnFastEnemy1`) 4.0))

(event `SpawnStandardEnemy1`
  (if (== (`self.UntilNextWave`) 0)
    (`AIBlueprintHelperLibrary.SpawnAIFromClass` "/Game/Common/Blueprints/BPI_EnemyStandard.BPI_EnemyStandard_C" null (`self.K2_GetActorLocation`) (struct) false null)))

(event `SpawnFastEnemy1`
  (if (== (`self.UntilNextWave`) 0)
    (`AIBlueprintHelperLibrary.SpawnAIFromClass` "/Game/Common/Blueprints/BPI_EnemyStandard.BPI_EnemyStandard_C" null (`self.K2_GetActorLocation`) (struct) false null)))

(fn `UserConstructionScript`)