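; Gate system Blueprint that shuts one of three gates as overlaps, presumably by enemies, accumulate at their check actors.
; All three checks increment one shared EnemyCounter without filtering the overlapping actor.
; Once it reaches the threshold, the triggering check's gate snaps up above its GatePoint and the counter resets.
; The other two gates then ease back to their GatePoint transforms via MoveComponentTo, leaving only the latest gate shut.
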(event `self.Gate1Check.OnActorBeginOverlap`
  (params (OverlappedActor :type "Actor Object Reference") (OtherActor :type "Actor Object Reference"))
  (bind _gatepoint2 (`self.GatePoint2`))
  (bind _gatepoint3 (`self.GatePoint3`))
  (bind _gate1 (`self.Gate1`))
  (bind _enemycounter (`self.EnemyCounter`))
  (bind (_returnvalue_x _returnvalue_y) (`KismetMathLibrary.BreakVector` (`self.K2_GetActorLocation` _gate1)))
  (bind (_returnvalue_x_2 _returnvalue_y_2 _returnvalue_z) (`KismetMathLibrary.BreakVector` (`self.K2_GetActorLocation` (`self.GatePoint1`))))
  ;[1 0.02 0.02] Overlap checks for all gate colliders. If => 3 the gate will move up from the ground and be shut and the counter is reset.
  (set `self.EnemyCounter` (+ _enemycounter 1))
  (if (>= _enemycounter 3)
    (`self.K2_SetActorLocation` _gate1 (`KismetMathLibrary.MakeVector` _returnvalue_x _returnvalue_y (+ _returnvalue_z 200.0)) false false)
    (set `self.EnemyCounter` 0)
    (`KismetSystemLibrary.PrintString` "Check 1")
    ;[1 0.02 0.02] When a gate is shut in the previous section. The other gates are reset to their original positions.
    (`|ExecutionSequence`
      (:`then_0`
        (`KismetSystemLibrary.MoveComponentTo` (`Actor.RootComponent` (`self.Gate2`)) (`self.K2_GetActorLocation` _gatepoint2) (`self.K2_GetActorRotation` _gatepoint2) true true 0.5))
      (:`then_1`
        (`KismetSystemLibrary.MoveComponentTo` (`Actor.RootComponent` (`self.Gate3`)) (`self.K2_GetActorLocation` _gatepoint3) (`self.K2_GetActorRotation` _gatepoint3) true true 0.5)))))

(event `self.Gate2Check.OnActorBeginOverlap`
  (params (OverlappedActor :type "Actor Object Reference") (OtherActor :type "Actor Object Reference"))
  (bind _gatepoint1 (`self.GatePoint1`))
  (bind _gatepoint3 (`self.GatePoint3`))
  (bind _gate2 (`self.Gate2`))
  (bind _enemycounter (`self.EnemyCounter`))
  (bind (_returnvalue_x _returnvalue_y) (`KismetMathLibrary.BreakVector` (`self.K2_GetActorLocation` _gate2)))
  (bind (_returnvalue_x_2 _returnvalue_y_2 _returnvalue_z) (`KismetMathLibrary.BreakVector` (`self.K2_GetActorLocation` (`self.GatePoint2`))))
  ;[1 0.02 0.02] Overlap checks for all gate colliders. If => 3 the gate will move up from the ground and be shut and the counter is reset.
  (set `self.EnemyCounter` (+ _enemycounter 1))
  (if (>= _enemycounter 3)
    (`self.K2_SetActorLocation` _gate2 (`KismetMathLibrary.MakeVector` _returnvalue_x _returnvalue_y (+ _returnvalue_z 200.0)) false false)
    (set `self.EnemyCounter` 0)
    (`KismetSystemLibrary.PrintString` "Check 2")
    ;[1 0.02 0.02] When a gate is shut in the previous section. The other gates are reset to their original positions.
    (`|ExecutionSequence`
      (:`then_0`
        (`KismetSystemLibrary.MoveComponentTo` (`Actor.RootComponent` (`self.Gate1`)) (`self.K2_GetActorLocation` _gatepoint1) (`self.K2_GetActorRotation` _gatepoint1) true true 0.5))
      (:`then_1`
        (`KismetSystemLibrary.MoveComponentTo` (`Actor.RootComponent` (`self.Gate3`)) (`self.K2_GetActorLocation` _gatepoint3) (`self.K2_GetActorRotation` _gatepoint3) true true 0.5)))))

(event `self.Gate3Check.OnActorBeginOverlap`
  (params (OverlappedActor :type "Actor Object Reference") (OtherActor :type "Actor Object Reference"))
  (bind _gate3 (`self.Gate3`))
  (bind _gatepoint1 (`self.GatePoint1`))
  (bind _gatepoint2 (`self.GatePoint2`))
  (bind _enemycounter (`self.EnemyCounter`))
  (bind (_returnvalue_x _returnvalue_y _returnvalue_z) (`KismetMathLibrary.BreakVector` (`self.K2_GetActorLocation` (`self.GatePoint3`))))
  (bind (_returnvalue_x_2 _returnvalue_y_2) (`KismetMathLibrary.BreakVector` (`self.K2_GetActorLocation` _gate3)))
  ;[1 0.02 0.02] Overlap checks for all gate colliders. If => 3 the gate will move up from the ground and be shut and the counter is reset.
  (set `self.EnemyCounter` (+ _enemycounter 1))
  (if (>= _enemycounter 3)
    (`self.K2_SetActorLocation` _gate3 (`KismetMathLibrary.MakeVector` _returnvalue_x_2 _returnvalue_y_2 (+ _returnvalue_z 200.0)) false false)
    (set `self.EnemyCounter` 0)
    (`KismetSystemLibrary.PrintString` "Check 3")
    ;[1 0.02 0.02] When a gate is shut in the previous section. The other gates are reset to their original positions.
    (`|ExecutionSequence`
      (:`then_0`
        (`KismetSystemLibrary.MoveComponentTo` (`Actor.RootComponent` (`self.Gate2`)) (`self.K2_GetActorLocation` _gatepoint2) (`self.K2_GetActorRotation` _gatepoint2) true true 0.5))
      (:`then_1`
        (`KismetSystemLibrary.MoveComponentTo` (`Actor.RootComponent` (`self.Gate1`)) (`self.K2_GetActorLocation` _gatepoint1) (`self.K2_GetActorRotation` _gatepoint1) true true 0.5)))))

(fn `UserConstructionScript`)